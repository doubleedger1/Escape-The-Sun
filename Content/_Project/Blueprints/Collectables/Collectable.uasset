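; Collectable pickup actor that hovers, bobs and spins, and reports its type when collected.
; On BeginPlay a downward line trace places it above the surface below, then a FlipFlop alternately plays and reverses a timeline to bob it around that spot.
; Tick applies constant yaw rotation.
; CollectObject shows a type-named "Collected!" widget, destroys the actor, plays the pickup sound and returns the collectable type.
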(event `self.ReceiveBeginPlay`
  (bind _returnvalue (`self.K2_GetActorLocation`))
  ;[1 1 1] Set Start Position
  (bind _outhit (`KismetSystemLibrary.LineTraceSingleForObjects` _returnvalue (+ _returnvalue (0.0 0.0 -1000.0)) (`|MakeArray` "ObjectTypeQuery1" "ObjectTypeQuery2" "ObjectTypeQuery3" "ObjectTypeQuery4" "ObjectTypeQuery6" "ObjectTypeQuery5" :!type "EObjectTypeQuery Enum")))
  (`self.K2_SetActorLocation` (+ (`.Location` (`GameplayStatics.BreakHitResult` _outhit)) (0.0 0.0 100.0)))
  ;[1 1 1] Collectable Movement
  ;;[1 1 1] Make collectable bob
  (set `self.Height` (`self.K2_GetActorLocation`))
  (`/Engine/EditorBlueprintResources/StandardMacros.FlipFlop` :!label _label
    (:`A`
      (bind (_direction _height) (`Timeline|FloatingPowerup` :!via `PlayFromStart` :!label _label_2)
        (:`Update`
          (`self.K2_SetActorLocation` (+ (`KismetMathLibrary.MakeVector` 0.0 0.0 (* _height (`self.HeightVariation`))) (`self.Height`))))
        (:`Finished`
          (`KismetSystemLibrary.Delay` 0.0)
          (goto _label))))
    (:`B`
      (goto _label_2 :!via `Reverse`))))

(event `self.ReceiveTick`
  (params (DeltaSeconds :type "Float (single-precision)"))
  ;[1 1 1] Collectable Movement
  ;;[1 1 1] Rotate Collectable
  (`self.K2_AddActorWorldRotation` (`KismetMathLibrary.MakeRotator` 0.0 0.0 (* DeltaSeconds (`self.RotationSpeed`)))))

(fn `CollectObject`
  (params (NewParam :type "/Game/_Project/Blueprints/Character/ThirdPersonCharacter Object Reference"))
  (returns (CollectableType :type "/Game/_Project/Blueprints/Collectables/Collectables Enum"))
  (bind _returnvalue (`|CreateWidget` "/Game/_Project/UserInterface/CollectText.CollectText_C" (`GameplayStatics.GetPlayerController` 0)))
  (set `/Game/_Project/UserInterface/CollectText.Text` (`KismetTextLibrary.Conv_StringToText` (`KismetStringLibrary.Concat_StrStr` (`|GetEnumeratorNameAsString` (`self.CollectableType`)) " Collected!")) _returnvalue)
  (`UserWidget.AddToViewport` _returnvalue 0)
  (`self.K2_DestroyActor`)
  (`GameplayStatics.PlaySoundAtLocation` "/Game/_Project/Sounds/pickup.pickup" (`self.K2_GetActorLocation`))
  (return (`self.CollectableType`)))

(fn `UserConstructionScript`)