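; Projectile actor that damages trolls and greater spiders on contact.
; Tick moves it along local X at fixed speed without physics and silently destroys it when its lifetime expires.
; Capsule overlap runs a cast chain that ignores pickups, certain triggers, doors, other bullets and ThirdPersonCharacter.
; Any other hit destroys the bullet with a half-scale explosion and sound, calling Damage first on those two enemy types.
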(event `self.ReceiveTick`
  (params (DeltaSeconds :type "Float (single-precision)"))
  (set `self.Lifetime` (- (`self.Lifetime`) DeltaSeconds))
  (`self.K2_AddActorLocalOffset` (`KismetMathLibrary.MakeVector` (* DeltaSeconds 5000.0)))
  (if (< (`self.Lifetime`) 0.0)
    (`self.K2_DestroyActor`)))

(event `self.cap.OnComponentBeginOverlap`
  (params (OverlappedComponent :type "PrimitiveComponent Object Reference") (OtherActor :type "Actor Object Reference") (OtherComp :type "PrimitiveComponent Object Reference") (OtherBodyIndex :type Integer) (bFromSweep :type Boolean) (SweepResult :type "HitResult Structure (by ref)"))
  (cast `/Game/_Project/Blueprints/Collectables/Collectable` OtherActor
    (:`CastFailed`
      (cast `/Game/_Project/Blueprints/SequentialLightTrigger` OtherActor
        (:`CastFailed`
          (cast `/Game/_Project/Blueprints/Environment/door_Blueprint` OtherActor
            (:`CastFailed`
              (cast `/Game/_Project/Blueprints/RespawnTrigger` OtherActor
                (:`CastFailed`
                  (cast `/Game/_Project/Blueprints/Character/Bullet` OtherActor
                    (:`CastFailed`
                      (bind _astroll_bp (cast `/Game/_Project/Blueprints/Enemies/Troll/Troll_BP` OtherActor)
                        (:`then`
                          (`/Game/_Project/Blueprints/Enemies/Troll/Troll_BP.Damage` _astroll_bp 10.0))
                        (:`CastFailed`
                          (bind _asgreater_spider_bp (cast `/Game/_Project/Blueprints/Enemies/Great_Spider/Greater_Spider_BP` OtherActor)
                            (:`then`
                              (`/Game/_Project/Blueprints/Enemies/Great_Spider/Greater_Spider_BP.Damage` _asgreater_spider_bp 10.0))
                            (:`CastFailed`
                              (cast `/Game/_Project/Blueprints/Character/ThirdPersonCharacter` OtherActor
                                (:`CastFailed`
                                  _))))))
                      (`self.K2_DestroyActor`)
                      (bind _returnvalue (`GameplayStatics.SpawnEmitterAtLocation` "/Game/StarterContent/Particles/P_Explosion.P_Explosion" (`self.K2_GetActorLocation`)))
                      (`SceneComponent.SetRelativeScale3D` _returnvalue (0.5 0.5 0.5))
                      (`GameplayStatics.PlaySoundAtLocation` "/Game/_Project/Sounds/explode.explode" (`self.K2_GetActorLocation`)))))))))))))

(fn `UserConstructionScript`)