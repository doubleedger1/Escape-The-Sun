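; DestructWall is a breakable wall built on a destructible mesh component that shatters after repeated overlaps.
; Each begin-overlap on the mesh increments a Damage counter, regardless of what overlaps it.
; Once the counter passes its threshold, it applies damage to the mesh at the actor's location, then disables the mesh's collision after a short delay.
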(event `self.Moving_platform_up_and_down_DM.OnComponentBeginOverlap`
  (params (OverlappedComponent :type "PrimitiveComponent Object Reference") (OtherActor :type "Actor Object Reference") (OtherComp :type "PrimitiveComponent Object Reference") (OtherBodyIndex :type Integer) (bFromSweep :type Boolean) (SweepResult :type "HitResult Structure (by ref)"))
  (bind _output_get (set `self.damage` (+ (`self.damage`) 1.0)))
  (if (> _output_get 4.0)
    (`DestructibleComponent.ApplyDamage` (`self.Moving_platform_up_and_down_DM`) 5.0 (`self.K2_GetActorLocation`) (0.0 0.0 0.0) 0.0)
    (`KismetSystemLibrary.Delay` 2.0)
    (`PrimitiveComponent.SetCollisionEnabled` (`self.Moving_platform_up_and_down_DM`) "NoCollision")))

(fn `UserConstructionScript`)