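; ConsoleBlastOff is an interactive console Blueprint on PlanetOne whose button glow the player toggles with the E key.
; Overlapping its Box trigger enables input from player controller 0 and shows a Hint; leaving reverses both.
; While input is enabled, each E press runs a FlipFlop that swaps one ButtonBase material slot between green and red glowing materials, with no launch logic attached.
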(event `self.Box.OnComponentBeginOverlap`
  (params (OverlappedComponent :type "PrimitiveComponent Object Reference") (OtherActor :type "Actor Object Reference") (OtherComp :type "PrimitiveComponent Object Reference") (OtherBodyIndex :type Integer) (bFromSweep :type Boolean) (SweepResult :type "HitResult Structure (by ref)"))
  ;[1 1 1] When we entter the trigger volume enable input and show hint
  (`self.EnableInput` (`GameplayStatics.GetPlayerController` 0))
  (`SceneComponent.SetVisibility` (`self.Hint`) true false))

(event `self.Box.OnComponentEndOverlap`
  (params (OverlappedComponent :type "PrimitiveComponent Object Reference") (OtherActor :type "Actor Object Reference") (OtherComp :type "PrimitiveComponent Object Reference") (OtherBodyIndex :type Integer))
  ;[1 1 1] When we entter the trigger volume enable input and show hint
  (`self.DisableInput` (`GameplayStatics.GetPlayerController` 0))
  (`SceneComponent.SetVisibility` (`self.Hint`) false false))

(event `Key|E` :consume false
  (params (Key :type "Key Structure" :default "AnyKey"))
  (:`Pressed`
    (`/Engine/EditorBlueprintResources/StandardMacros.FlipFlop`
      (:`A`
        (`PrimitiveComponent.SetMaterial` (`self.buttonBase`) 2 "/Game/_Project/Models/SpaceShip/greenglowy.greenglowy"))
      (:`B`
        (`PrimitiveComponent.SetMaterial` (`self.buttonBase`) 2 "/Game/_Project/Models/SpaceShip/redglowy.redglowy")))))

(fn `UserConstructionScript`)