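; Clot Worm enemy Blueprint that chases the player and deals periodic damage at close range.
; While alive, Tick measures player distance, moves toward the player within a wider chase range and calls the character's Damage function on a one-second cooldown when near.
; Player overlap with JumpCol kills it, enabling mesh physics, then disabling capsule collision and destroying it after a short delay.
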(event `self.ReceiveTick`
  (params (DeltaSeconds :type "Float (single-precision)"))
  (if (`self.alive`)
    (set `self.DamageCountdown` (- (`self.DamageCountdown`) DeltaSeconds))
    (bind _range (`self.GetRange`))
    (if (and (< _range 500.0) (< (`self.DamageCountdown`) 0.0))
      (bind _asthird_person_character (cast `/Game/_Project/Blueprints/Character/ThirdPersonCharacter` (`GameplayStatics.GetPlayerPawn` 0)))
      (`/Game/_Project/Blueprints/Character/ThirdPersonCharacter.Damage` _asthird_person_character (`self.DamagePerSec`))
      (set `self.DamageCountdown` 1.0))
    (if (< _range 2000.0)
      (`NavigationSystem.SimpleMoveToActor` (`self.GetController`) (`GameplayStatics.GetPlayerCharacter` 0)))))

(event `self.jumpCol.OnComponentBeginOverlap`
  (params (OverlappedComponent :type "PrimitiveComponent Object Reference") (OtherActor :type "Actor Object Reference") (OtherComp :type "PrimitiveComponent Object Reference") (OtherBodyIndex :type Integer) (bFromSweep :type Boolean) (SweepResult :type "HitResult Structure (by ref)"))
  (cast `/Game/_Project/Blueprints/Character/ThirdPersonCharacter` OtherActor)
  (set `self.alive` false)
  (`PrimitiveComponent.SetSimulatePhysics` (`self.Mesh`) true)
  (`KismetSystemLibrary.Delay` 0.5)
  (`PrimitiveComponent.SetCollisionEnabled` (`self.CapsuleComponent`) "NoCollision")
  (`self.K2_DestroyActor`))

(fn `GetRange`
  (returns (Range :type "Float (double-precision)"))
  (return (`KismetMathLibrary.Abs` (`KismetMathLibrary.VSize` (- (`self.K2_GetActorLocation` (`GameplayStatics.GetPlayerCharacter` 0)) (`self.K2_GetActorLocation`))))))

(fn `UserConstructionScript`)