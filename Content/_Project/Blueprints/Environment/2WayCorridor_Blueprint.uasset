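; Two-way corridor environment actor with a spotlight that starts dark and flickers at random once switched on.
; BeginPlay hides the light, and the Turnon event shows it and sets the Visible flag that enables flickering.
; While that flag is set, each Tick has a roughly one-in-a-thousand chance to toggle the light, then toggle it again after a short random delay, so flicker frequency depends on frame rate.
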(event `self.ReceiveBeginPlay`
  (set `self.visible` false)
  (`SceneComponent.SetVisibility` (`self.SpotLight`) false false))

(event `self.ReceiveTick`
  (params (DeltaSeconds :type "Float (single-precision)"))
  (if (and (`self.visible`) (== (`KismetMathLibrary.RandomIntegerInRange` 0 1000) 1))
    (`SceneComponent.ToggleVisibility` (`self.SpotLight`) false)
    (`KismetSystemLibrary.Delay` (`KismetMathLibrary.RandomFloatInRange` 0.1 0.4))
    (`SceneComponent.ToggleVisibility` (`self.SpotLight`) false)))

(event `/Game/_Project/Blueprints/Light.TurnOn`
  (set `self.visible` true)
  (`SceneComponent.SetVisibility` (`self.SpotLight`) true false))

(fn `UserConstructionScript`)