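; Sliding double door that opens when the player's ThirdPersonCharacter enters its trigger box, unless it is Locked.
; Overlap plays a sound and runs the OpenDoors timeline, offsetting both panels along local Y from cached shut positions by OpenWidth; leaving reverses it.
; Tick compares the right panel's material with the Locked state and swaps slot 2 on both panels when they disagree.
; MoveDoors is an empty stub.
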(event `self.ReceiveBeginPlay`
  (set `self.doorLeftShutPos` (`SceneComponent.RelativeLocation` (`self.doorLeft`)))
  (set `self.doorRightShutPos` (`SceneComponent.RelativeLocation` (`self.doorRight`))))

(event `self.ReceiveTick`
  (params (DeltaSeconds :type "Float (single-precision)"))
  (bind _locked (`self.locked`))
  ;[1 1 1] Set correct mat
  (bind _locked_2 (`self.GetLockedMaterialSet`))
  (if _locked_2
    (if (not _locked)
      (`self.SetMat` (`self.UnlockedMat`)))
    (elif _locked
      (`self.SetMat` (`self.LockedMat`)))))

(event `self.Box.OnComponentBeginOverlap`
  (params (OverlappedComponent :type "PrimitiveComponent Object Reference") (OtherActor :type "Actor Object Reference") (OtherComp :type "PrimitiveComponent Object Reference") (OtherBodyIndex :type Integer) (bFromSweep :type Boolean) (SweepResult :type "HitResult Structure (by ref)"))
  (bind (_doorleftshutpos_x _doorleftshutpos_y _doorleftshutpos_z) (`KismetMathLibrary.BreakVector` (`self.doorLeftShutPos`)))
  (bind (_doorrightshutpos_x _doorrightshutpos_y) (`KismetMathLibrary.BreakVector` (`self.doorRightShutPos`)))
  (bind (_doorrightshutpos_x_2 _doorrightshutpos_y_2 _doorrightshutpos_z) (`KismetMathLibrary.BreakVector` (`self.doorRightShutPos`)))
  (bind (_doorleftshutpos_x_2 _doorleftshutpos_y_2) (`KismetMathLibrary.BreakVector` (`self.doorLeftShutPos`)))
  (cast `/Game/_Project/Blueprints/Character/ThirdPersonCharacter` OtherActor)
  (if (not (`self.locked`))
    (`GameplayStatics.PlaySoundAtLocation` null (`self.K2_GetActorLocation`))
    (bind (_direction _y) (`Timeline|OpenDoors` :!label _label)
      (:`Update`
        (`SceneComponent.K2_SetRelativeLocation` (`self.doorRight`) (`KismetMathLibrary.MakeVector` _doorrightshutpos_x_2 (+ (* _y (`self.OpenWidth`) -1.0) _doorrightshutpos_y) _doorrightshutpos_z) false false)
        (`SceneComponent.K2_SetRelativeLocation` (`self.doorLeft`) (`KismetMathLibrary.MakeVector` _doorleftshutpos_x (+ (* _y (`self.OpenWidth`)) _doorleftshutpos_y_2) _doorleftshutpos_z) false false)))))

(event `self.Box.OnComponentEndOverlap`
  (params (OverlappedComponent :type "PrimitiveComponent Object Reference") (OtherActor :type "Actor Object Reference") (OtherComp :type "PrimitiveComponent Object Reference") (OtherBodyIndex :type Integer))
  (cast `/Game/_Project/Blueprints/Character/ThirdPersonCharacter` OtherActor)
  (goto _label :!via `Reverse`))

(fn `GetLockedMaterialSet`
  (returns (Locked :type Boolean))
  (return (== (`PrimitiveComponent.GetMaterial` (`self.doorRight`) 2) (`self.LockedMat`))))

(fn `MoveDoors`
  (params (Open :type Boolean)))

(fn `SetMat`
  (params (Mat :type "Material Object Reference"))
  (`PrimitiveComponent.SetMaterial` (`self.doorRight`) 2 Mat)
  (`PrimitiveComponent.SetMaterial` (`self.doorLeft`) 2 Mat))

(fn `UserConstructionScript`)